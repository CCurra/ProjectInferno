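; ShotgunBP is a shotgun weapon Blueprint for a zombie game that fires a spread of projectiles.
; Its Fire event loops to spawn several scaled-down Projectile_Base actors at an offset from the SGMarker component, rotated into the marker's facing.
; Each pellet gets random pitch and yaw deviation from the marker's rotation, and spawning adjusts for collisions but always succeeds.
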(event Custom|Fire
  (bind _sg_marker (Variables|Default|GetSG_Marker))
  (bind _returnvalue (Transformation|GetWorldRotation _sg_marker))
  (bind (_roll _pitch _yaw) (Math|Rotator|BreakRotator _returnvalue))
  (for _index (range 0 10)
    (Game|SpawnActorfromClass "/Game/ZombieGame/Blueprints/Weapons/Shotgun/Projectile_Base.Projectile_Base_C" (Math|Transform|MakeTransform (+ (Transformation|GetWorldLocation (Variables|Default|GetSG_Marker)) (Math|Vector|RotateVector (Variables|Default|GetNewVar_0) _returnvalue)) (Math|Rotator|MakeRotator _roll (+ _pitch (Math|Random|RandomFloatinRange -1e+01 1e+01)) (+ _yaw (Math|Random|RandomFloatinRange -1e+01 1e+01))) "0.300000,0.300000,0.300000") "AdjustIfPossibleButAlwaysSpawn" 0 0)))

(event EventBeginPlay)

(event Collision|EventActorBeginOverlap
  (params (OtherActor :type Actor%20Object%20Reference)))

(event EventTick
  (params (DeltaSeconds :type Float%20%28single-precision%29)))

(fn ConstructionScript)