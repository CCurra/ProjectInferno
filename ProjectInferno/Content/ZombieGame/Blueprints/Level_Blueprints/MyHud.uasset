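; MyHud is a HUD Blueprint that draws a full-screen overlay while the player is in a loading state.
; On each DrawHUD it converts the screen size to a vector and casts player character 0 to Player.
; When that Player's Loading flag is true, it draws a simple material sized to the screen.
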(event EventBeginPlay)

(event Collision|EventActorBeginOverlap
  (params (OtherActor :type Actor%20Object%20Reference)))

(event EventTick
  (params (DeltaSeconds :type Float%20%28single-precision%29)))

(event EventDrawHUD
  (params (SizeX :type Integer) (SizeY :type Integer))
  ;[1 1 1] Playing Screen Size
  (Variables|Default|SetScreen-dimentions (Math|Vector2D|MakeVector2D (Math|Conversions|ToFloat(Integer) SizeX) (Math|Conversions|ToFloat(Integer) SizeY)))
  (bind _asplayer (Utilities|Casting|CastToPlayer (Game|GetPlayerCharacter 0)))
  (if (Variables|/Game/ZombieGame/Blueprints/Level_Blueprints/Player.Player_C|GetLoading _asplayer)
    (Class|HUD|DrawMaterialSimple 0 0.0 0.0 (.X (Math|Vector2D|BreakVector2D (Variables|Default|GetScreen-dimentions))) (.Y (Math|Vector2D|BreakVector2D (Variables|Default|GetScreen-dimentions))) 1.0 false)))

(fn ConstructionScript)